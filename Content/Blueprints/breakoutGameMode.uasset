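; Game mode for a Breakout game that builds the brick wall when play begins.
; Two nested loops spawn Brick actors in a fixed grid on the X=0 plane, with columns spread along Y and rows stepping down in Z.
; Grid size, spacing and origin are hardcoded in the spawn math, and the file holds no other game logic.
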(event EventBeginPlay
  (for _index (range 0 3)
    (for _index_2 (range 0 8)
      (Game|SpawnActorfromClass "/Game/Blueprints/Brick.Brick_C" (Math|Transform|MakeTransform (Math|Vector|MakeVector 0.0 (Math|Conversions|ToFloat(Integer) (+ (* _index_2 50) -200)) (Math|Conversions|ToFloat(Integer) (- 90 (* _index 25))))) "Undefined" 0 0))))

(fn ConstructionScript)